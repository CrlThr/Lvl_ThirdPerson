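; BP_MasterTrigger is a box trigger that acts as either a death zone or a checkpoint for the player, selected by its TriggerType.
; It caches the player character as BP_Player on BeginPlay and responds only when that actor overlaps the box.
; A checkpoint stores its own location as the player's RespawnLoc and prints a debug message.
; A death zone moves the player back to that stored location.
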(event OnComponentBeginOverlap(Box)
  (params (OverlappedComponent :type Primitive%20Component%20Object%20Reference) (OtherActor :type Actor%20Object%20Reference) (OtherComp :type Primitive%20Component%20Object%20Reference) (OtherBodyIndex :type Integer) (bFromSweep :type Boolean) (SweepResult :type Hit%20Result%20Structure%20%28by%20ref%29))
  (bind _as_bp_player (Variables|Default|GetAs%20BP%20Player))
  (if (== OtherActor (Variables|Default|GetAs%20BP%20Player))
    (switch Utilities|FlowControl|Switch|SwitchonE_TriggerType (Variables|Default|GetTriggerType)
      (:NewEnumerator0
        (CallFunction|DeathZoneEvent _as_bp_player (Variables|/Game/Blueprints/Characters/BP_Player.BP_Player_C|GetRespawnLoc _as_bp_player)))
      (:NewEnumerator1
        (CallFunction|CheckPoint (Variables|Default|GetAs%20BP%20Player))))))

(event Custom|DeathZoneEvent
  (params (PlayerReference :type Actor%20Object%20Reference) (RespawnLocation :type Vector))
  (Transformation|SetActorLocation PlayerReference RespawnLocation false false))

(event EventBeginPlay
  (bind _asbp_player (Utilities|Casting|CastToBP_Player (Game|GetPlayerCharacter 0)))
  (Variables|Default|SetAs%20BP%20Player _asbp_player))

(fn ConstructionScript)

(fn CheckPoint
  (params (PlayerReference :type BP%20Player%20Object%20Reference))
  (Development|PrintString "CheckPoint")
  (Variables|/Game/Blueprints/Characters/BP_Player.BP_Player_C|SetRespawnLoc PlayerReference (Transformation|GetActorLocation)))